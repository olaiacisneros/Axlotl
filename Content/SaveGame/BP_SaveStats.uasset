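; BP_SaveStats is a save object holding player and run stats such as health, money, weapon choice, room progress, dash and special-attack settings, upgrades and a camera shake option.
; Its DefaultValues function resets these to starting values, setting MaxHealth from the fresh Health.
; It then writes itself to the hardcoded "Slot1" save slot, so the reset persists immediately.
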(fn DefaultValues
  (bind _output_get (Variables|Default|SetHealth 1.2e+02))
  (Variables|Default|SetRoomCounter 0.0)
  (Variables|Default|SetWeaponSelected 1.0)
  (Variables|Default|SetRoomNumber 0)
  (Variables|Default|SetCameraShake true)
  (Variables|Default|SetMoney 100)
  (Variables|Default|SetMaxHealth _output_get)
  (Variables|Default|SetRoomLife false)
  (Variables|Default|SetCoolDownSpecialAttack 1.5)
  (Variables|Default|SetDashCounter 1)
  (Variables|Default|SetUpgradeArray (Utilities|Array|MakeArray 10))
  (SaveGame|SaveGametoSlot self "Slot1"))