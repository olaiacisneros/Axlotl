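; BP_Alabarda is a halberd weapon actor that spawns Niagara effects for light attacks, heavy attacks and impacts.
; The light and heavy functions attach a trail to the StaticMesh, centered between the VFX_Top and VFX_Bottom sockets and aligned along them, with TrailWidth set to their distance.
; The impact function attaches its effect at the VFX_Impact socket.
; The event graph and construction script are empty, so nothing here calls these functions.
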(event EventBeginPlay)

(event Collision|EventActorBeginOverlap
  (params (OtherActor :type Actor%20Object%20Reference)))

(event EventTick
  (params (DeltaSeconds :type Float%20%28single-precision%29)))

(fn ConstructionScript)

(fn SpawnVFXLightAtack
  (bind _staticmesh (Variables|Default|GetStaticMesh))
  (bind _returnvalue (Transformation|GetSocketLocation _staticmesh "VFX_Bottom"))
  (bind _returnvalue_2 (Transformation|GetSocketLocation _staticmesh "VFX_Top"))
  (bind _returnvalue_3 (- _returnvalue_2 _returnvalue))
  (bind _returnvalue_4 (Niagara|SpawnSystemAttached "/Game/VFX/NS_Weapon1_Light.NS_Weapon1_Light" _staticmesh "None" (/ (+ _returnvalue_2 _returnvalue) 2.0) (Math|Rotator|MakeRotfromZ _returnvalue_3) "KeepWorldPosition" false))
  (Effects|Components|ParticleSystem|SetFloatParameter _returnvalue_4 "TrailWidth" (Math|Vector|VectorLength _returnvalue_3)))

(fn SpawnVFXHeavyAtack
  (bind _staticmesh (Variables|Default|GetStaticMesh))
  (bind _returnvalue (Transformation|GetSocketLocation _staticmesh "VFX_Bottom"))
  (bind _returnvalue_2 (Transformation|GetSocketLocation _staticmesh "VFX_Top"))
  (bind _returnvalue_3 (- _returnvalue_2 _returnvalue))
  (bind _returnvalue_4 (Niagara|SpawnSystemAttached "/Game/VFX/NS_Weapon1_heavy.NS_Weapon1_heavy" _staticmesh "None" (/ (+ _returnvalue_2 _returnvalue) 2.0) (Math|Rotator|MakeRotfromZ _returnvalue_3) "KeepWorldPosition" false))
  (Effects|Components|ParticleSystem|SetFloatParameter _returnvalue_4 "TrailWidth" (Math|Vector|VectorLength _returnvalue_3)))

(fn SpawnVFXImpact
  (bind _staticmesh (Variables|Default|GetStaticMesh))
  (Niagara|SpawnSystemAttached "/Game/VFX/NS_Impact.NS_Impact" _staticmesh "None" (Transformation|GetSocketLocation _staticmesh "VFX_Impact") "0, 0, 0" "KeepWorldPosition" false))