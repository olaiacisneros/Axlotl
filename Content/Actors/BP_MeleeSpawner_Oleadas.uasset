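; BP_MeleeSpawner_Oleadas is a spawner for random melee enemies, tied to the BP_TimeCounter_Oleadas timer found at BeginPlay.
; Each Tick compares its Time threshold with the counter, spawning one BP_Enemy_Melee_Random when the threshold is greater and the Spawn flag is set.
; Spawning clears the flag and sets Time to the counter value plus 80% of the old threshold.
; The flag re-arms whenever the threshold is not above the counter.
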(event EventBeginPlay
  (bind _returnvalue (Actor|GetActorOfClass "/Game/Actors/BP_TimeCounter_Oleadas.BP_TimeCounter_Oleadas_C"))
  (Variables|Default|SetTimer _returnvalue))

(event EventTick
  (params (DeltaSeconds :type Float%20%28single-precision%29))
  (bind _totalseconds (Default|GetTime (Variables|Default|GetTimer)))
  (if (> (Variables|Default|GetTime) _totalseconds)
    (if (Variables|Default|GetSpawn)
      (Variables|Default|SetSpawn false)
      (Development|PrintString "MeleeSpawner: Spawn")
      (Game|SpawnActorfromClass "/Game/Enemies/BaseEnemy/BP_Enemy_Melee_Random.BP_Enemy_Melee_Random_C" (Math|Transform|MakeTransform "0, 0, 0" "0, 0, 0" "1.000000,1.000000,1.000000") "Undefined" "MultiplyWithRoot" 0 0)
      (bind _totalseconds_2 (Default|GetTime (Variables|Default|GetTimer)))
      (Variables|Default|SetTime (+ _totalseconds_2 (* (Variables|Default|GetTime) 0.8))))
    (else
      (Variables|Default|SetSpawn true))))

(fn ConstructionScript)