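; BP_SpawnerRagedOleadas is a one-shot, timed spawner for a ranged enemy, BP_Enemy_RangedCordoba, in wave (oleadas) gameplay.
; On BeginPlay it finds and caches the level's BP_TimeCounter_Oleadas.
; Each Tick it polls that counter until the elapsed time exceeds its Time variable.
; A DoOnce then spawns the enemy at the spawner's location, and the spawner destroys itself.
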(event EventBeginPlay
  (bind _returnvalue (Actor|GetActorOfClass "/Game/Actors/BP_TimeCounter_Oleadas.BP_TimeCounter_Oleadas_C"))
  (Variables|Default|SetTimeCounter _returnvalue))

(event Collision|EventActorBeginOverlap
  (params (OtherActor :type Actor%20Object%20Reference)))

(event EventTick
  (params (DeltaSeconds :type Float%20%28single-precision%29))
  (bind _totalseconds (Default|GetTime (Variables|Default|GetTimeCounter)))
  (if (> _totalseconds (Variables|Default|GetTime))
    (Utilities|FlowControl|DoOnce false
      (:Completed
        (Game|SpawnActorfromClass "/Game/Enemies/BaseEnemy/BP_Enemy_RangedCordoba.BP_Enemy_RangedCordoba_C" (Math|Transform|MakeTransform (Transformation|GetActorLocation) "0, 0, 0" "1.000000,1.000000,1.000000") "Undefined" "MultiplyWithRoot" 0 0)
        (Actor|DestroyActor)))))

(fn ConstructionScript)