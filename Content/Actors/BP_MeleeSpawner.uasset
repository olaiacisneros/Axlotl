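; BP_MeleeSpawner is a placed actor that periodically spawns random melee enemies (BP_Enemy_Melee_Random) at its own location.
; BeginPlay starts a timer with the interval set by Time and looping controlled by the Spawn flag.
; Each tick of the timer spawns an enemy and increments ContadorEnemigos.
; The timer pauses once that count exceeds LimiteEnemigos, so a looping spawner produces one more than the limit.
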(event Custom|Spawn_Melee
  (Game|SpawnActorfromClass "/Game/Enemies/BaseEnemy/BP_Enemy_Melee_Random.BP_Enemy_Melee_Random_C" (Math|Transform|MakeTransform (Transformation|GetActorLocation) "0, 0, 0" "1.000000,1.000000,1.000000") "Undefined" "MultiplyWithRoot" 0 0)
  (Math|Float|IncrementFloat (Variables|Default|GetContadorEnemigos)
    (:%20%20
      (if (not (<= (Variables|Default|GetContadorEnemigos) (Variables|Default|GetLimiteEnemigos)))
        (Utilities|Time|PauseTimerbyHandle (Variables|Default|GetEventTimer))))))

(event EventBeginPlay
  (bind _returnvalue (Utilities|Time|SetTimerbyEvent (delegate Custom|Spawn_Melee) (Variables|Default|GetTime) (Variables|Default|GetSpawn)))
  (Variables|Default|SetEventTimer _returnvalue))

(fn ConstructionScript)