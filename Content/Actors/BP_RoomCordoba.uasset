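; BP_RoomCordoba is a room-transition trigger that moves the player into the next combat level.
; On player overlap it saves BP_Axololt's data through GI_Music, plays a shutter sound and the WB_RoomChange fade, then waits briefly.
; GI_Music's elapsed time selects the destination: Sala_Batalla below the threshold, Sala_Oleadas otherwise.
; Helpers for random room choice and saving/loading the upgrade array via BP_SaveStats are not called from the event graph.
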(event OnComponentBeginOverlap(Trigger)
  (params (OverlappedComponent :type Primitive%20Component%20Object%20Reference) (OtherActor :type Actor%20Object%20Reference) (OtherComp :type Primitive%20Component%20Object%20Reference) (OtherBodyIndex :type Integer) (bFromSweep :type Boolean) (SweepResult :type Hit%20Result%20Structure%20%28by%20ref%29))
  (if (Actor|ActorHasTag OtherActor "Player")
    (bind _asgi_music (Utilities|Casting|CastToGI_Music (Game|GetGameInstance)))
    (bind _minutes (Default|TimePassed _asgi_music))
    ;[1 1 1] Esto para guardar IMPORTANTE
    (bind _playersave (Default|GetPlayerSave (Variables|Default|Get%20BP%20Axololt)))
    (Default|SavePlayer _asgi_music _playersave false)
    (Audio|PlaySound2D "/Engine/VREditor/Sounds/UI/Camera_Shutter.Camera_Shutter" 1.0 1.0 0.0 0 0)
    (bind _returnvalue (UserInterface|CreateWidget "/Game/Widgets/WB_RoomChange.WB_RoomChange_C"))
    (UserInterface|Viewport|AddtoViewport _returnvalue 0)
    (Default|FadeEvent _returnvalue)
    (Utilities|FlowControl|Delay 1.0)
    (if (< _minutes 5.0)
      (Game|OpenLevel(byName) "Sala_Batalla")
      (else
        (Game|OpenLevel(byName) "Sala_Oleadas")))))

(event EventBeginPlay
  (bind _asbp_axololt (Utilities|Casting|CastToBP_Axololt (Game|GetPlayerCharacter 0)))
  (Variables|Default|Set%20BP%20Axololt _asbp_axololt))

(fn ConstructionScript)

(fn SalaRandom
  (return (Math|Conversions|ToByte(Integer) (Math|Random|RandomIntegerinRange 0 2))))

(fn UpgradeRandom)

(fn SaveGame
  (params (Slot%20Name :type String))
  (bind _returnvalue (SaveGame|DoesSaveGameExist (Variables|Default|GetSlot%20Name%20Save)))
  (if _returnvalue
    (SaveGame|CreateSaveGameObject "/Game/SaveGame/BP_SaveStats.BP_SaveStats_C")
    (bind _returnvalue_2 (SaveGame|LoadGamefromSlot (Variables|Default|GetSlot%20Name%20Save)))
    (Variables|Default|SetSave%20REF _returnvalue_2)
    (else
      (bind _returnvalue_3 (SaveGame|CreateSaveGameObject "/Game/SaveGame/BP_SaveStats.BP_SaveStats_C"))
      (Variables|Default|SetSave%20REF _returnvalue_3)))
  (bind _asbp_save_stats (Utilities|Casting|CastToBP_SaveStats (Variables|Default|GetSave%20REF)))
  (Variables|/Game/SaveGame/BP_SaveStats.BP_SaveStats_C|SetUpgradeArray _asbp_save_stats (Variables|Default|GetUpgradesArray))
  (bind _returnvalue_4 (SaveGame|SaveGametoSlot _asbp_save_stats Slot%20Name))
  (Development|PrintText (Utilities|Text|FormatText "RoomChange: Saved {1}" _returnvalue_4)))

(fn LoadGame
  (params (Slot%20Name :type String))
  (bind _returnvalue (SaveGame|DoesSaveGameExist Slot%20Name))
  (if _returnvalue
    (Development|PrintString "RoomChange: True")
    (bind _returnvalue_2 (SaveGame|LoadGamefromSlot Slot%20Name))
    (bind _asbp_save_stats (Utilities|Casting|CastToBP_SaveStats _returnvalue_2))
    (Variables|Default|SetUpgradesArray (Variables|/Game/SaveGame/BP_SaveStats.BP_SaveStats_C|GetUpgradeArray _asbp_save_stats))
    (else
      (Development|PrintString "RoomChange: False")
      (SaveGame|CreateSaveGameObject "/Game/SaveGame/BP_SaveStats.BP_SaveStats_C")
      (Development|PrintString "RoomChange: Create Save Game")
      (CallFunction|SaveGame (Variables|Default|GetSlot%20Name%20Save)))))