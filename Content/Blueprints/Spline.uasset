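; Spline actor that builds a repeated mesh along an editable spline, with no active runtime logic.
; The construction script steps along the spline in Section-length intervals, adding a SplineMeshComponent with the configured mesh and material for each.
; Each segment takes local-space positions and tangents sampled by distance, with tangent length clamped to Section so the mesh bends cleanly along the curve.
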(event EventBeginPlay)

(event Collision|EventActorBeginOverlap
  (params (OtherActor :type Actor%20Object%20Reference)))

(event EventTick
  (params (DeltaSeconds :type Float%20%28single-precision%29)))

(fn ConstructionScript
  (bind _spline (Variables|Default|GetSpline))
  (bind _section (Variables|Default|GetSection))
  (for _index (range 0 (Math|Float|Truncate (/ (Spline|GetSplineLength (Variables|Default|GetSpline)) (Variables|Default|GetSection))))
    (Variables|Default|SetIndex _index)
    (bind _returnvalue (AddComponent|AddSplineMeshComponent false))
    (Rendering|Material|SetMaterial _returnvalue 0 (Variables|Default|GetSpline%20Material))
    (Components|StaticMesh|SetStaticMesh _returnvalue (Variables|Default|GetSpline%20Mesh))
    (SplineMesh|SetForwardAxis _returnvalue "X" true)
    (SplineMesh|SetStartandEnd _returnvalue (Spline|GetLocationatDistanceAlongSpline _spline (* (Variables|Default|GetIndex) _section) "Local") (Math|Vector|ClampVectorSize (Spline|GetTangentatDistanceAlongSpline _spline (* (Variables|Default|GetIndex) _section) "Local") 0.0 _section) (Spline|GetLocationatDistanceAlongSpline _spline (* (+ (Variables|Default|GetIndex) 1) _section) "Local") (Math|Vector|ClampVectorSize (Spline|GetTangentatDistanceAlongSpline _spline (* (+ (Variables|Default|GetIndex) 1) _section) "Local") 0.0 _section) true :!class /Script/Engine.SplineMeshComponent)))