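; BP_Enemy3 is a ranged enemy that turns to face the Axololt pawn when its PawnSensing component sees it and shoots at it.
; On each sighting it snaps its rotation toward the target, then spawns a BP_ProjectileEnemy3 at the SpawnProjectile component's transform.
; A CanAttack flag and a ShootCooldown delay limit the fire rate, while rotation still updates on every sighting.
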(event OnSeePawn(PawnSensing)
  (params (Pawn :type Pawn%20Object%20Reference))
  (bind _asaxololt (Utilities|Casting|CastToAxololt Pawn))
  (Transformation|SetActorRotation (Math|Rotator|FindRelativeLookatRotation (Math|Conversions|ToTransform(Vector) (Transformation|GetActorLocation)) (Transformation|GetActorLocation _asaxololt)))
  (if (Variables|Default|GetCanAttack)
    (Game|SpawnActorfromClass "/Game/Actors/BP_ProjectileEnemy3.BP_ProjectileEnemy3_C" (Transformation|GetWorldTransform (Variables|Default|GetSpawnProjectile)) "Undefined" "MultiplyWithRoot" 0 0)
    (Variables|Default|SetCanAttack false)
    (Utilities|FlowControl|Delay (Variables|Default|GetShoot_Cooldown))
    (Variables|Default|SetCanAttack true)))

(event EventBeginPlay)

(event Collision|EventActorBeginOverlap
  (params (OtherActor :type Actor%20Object%20Reference)))

(event EventTick
  (params (DeltaSeconds :type Float%20%28single-precision%29)))

(fn ConstructionScript)