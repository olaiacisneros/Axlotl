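; Melee enemy Blueprint that splits into two BP_MiniEnemy actors on death.
; Tick pushes its health to a widget health bar.
; Attack plays a montage, damages the AI controller's AttackTarget as the montage starts, and calls AttackEnd when it completes or is interrupted.
; Lethal damage runs once: it stops movement, starts the death montage, spawns the minions at two sphere components, then destroys itself after a delay.
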(event EventBeginPlay)

(event Collision|EventActorBeginOverlap
  (params (OtherActor :type Actor%20Object%20Reference)))

(event EventTick
  (params (DeltaSeconds :type Float%20%28single-precision%29))
  ;[1 0.9142 0.2333] Event tick
  (bind _aswb_melee_enemy (Utilities|Casting|CastToWB_MeleeEnemy (UserInterface|GetWidget (Variables|Default|GetHealthBar))))
  (Progress|SetPercent (Variables|/Game/Widgets/Enemies/WB_MeleeEnemy.WB_MeleeEnemy_C|GetHealthBar _aswb_melee_enemy) (/ (Variables|Default|GetEnemy_Health) 1e+02)))

(event EventAttack
  ;[1 0 0.8377] Ataque
  (Animation|Montage|PlayMontage (Variables|Character|GetMesh) "/Game/Enemies/BaseEnemy/Animations/Enemy1/Anim_BP/AM_Attack.AM_Attack"
    (:then
      (bind _asaicontroller_base_enemy (Utilities|Casting|CastToAIController_BaseEnemy (AI|GetAIController self)))
      (bind _attack_target (Variables|/Game/Enemies/BaseEnemy/AI/AIController_BaseEnemy.AIController_BaseEnemy_C|GetAttack%20Target _asaicontroller_base_enemy)
        (:then
          (Game|Damage|ApplyDamage _attack_target (Variables|Default|GetEnemy_Dmg) 0 0))
        (:else)))
    (:OnCompleted
      (Default|CallAttackEnd :!label _label))
    (:OnInterrupted
      (goto _label))))

(event Game|Damage|EventAnyDamage
  (params (Damage :type Float%20%28single-precision%29) (DamageType :type Damage%20Type%20Object%20Reference) (InstigatedBy :type Controller%20Object%20Reference) (DamageCauser :type Actor%20Object%20Reference))
  ;[1 0 0] Recibir daño
  (bind _output_get (Variables|Default|SetEnemy_Health (- (Variables|Default|GetEnemy_Health) Damage)))
  (if (<= _output_get 0.0)
    (Utilities|FlowControl|DoOnce false
      (:Completed
        (Variables|Default|SetbUseControllerRotationYaw false)
        (Pawn|Components|CharacterMovement|DisableMovement (Variables|Character|GetCharacterMovement))
        (Animation|Montage|PlayMontage (Variables|Character|GetMesh) "/Game/Enemies/BaseEnemy/Animations/Enemy1/Anim_BP/AM_Death.AM_Death"
          (:then
            (Game|SpawnActorfromClass "/Game/Enemies/BaseEnemy/BP_MiniEnemy.BP_MiniEnemy_C" (Transformation|GetWorldTransform (Variables|Default|GetSphere)) "Undefined" "MultiplyWithRoot" 0 0)
            (Game|SpawnActorfromClass "/Game/Enemies/BaseEnemy/BP_MiniEnemy.BP_MiniEnemy_C" (Transformation|GetWorldTransform (Variables|Default|GetSphere1)) "Undefined" "MultiplyWithRoot" 0 0)
            (Utilities|FlowControl|Delay 3.0)
            (Actor|DestroyActor)))))))

(fn ConstructionScript
  (|CallParentFunction))

(fn GetHealth
  (return 0.0))