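; BP_MiniEnemy is a small melee enemy with a health bar widget updated every Tick and a skeleton component attached to its head socket.
; Attack plays a montage, immediately damages the AI controller's AttackTarget, and signals AttackEnd on completion or interruption.
; Taking damage spawns floating numbers and launches it along the player's forward vector; at zero health it stops moving, plays death and destroys itself.
; GetHealth and SetMovementSpeed are stubs.
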(event EventBeginPlay
  ;[0.09435 1 0.07239] BeginPlay
  (Transformation|AttachComponentToComponent (Variables|Default|GetEsqueleto) (Variables|Character|GetMesh) "HeadSocket" "SnapToTarget" "SnapToTarget" "SnapToTarget" true))

(event Collision|EventActorBeginOverlap
  (params (OtherActor :type Actor%20Object%20Reference)))

(event EventTick
  (params (DeltaSeconds :type Float%20%28single-precision%29))
  ;[1 0.8721 0.1784] Event tick
  (bind _aswb_melee_enemy (Utilities|Casting|CastToWB_MeleeEnemy (UserInterface|GetWidget (Variables|Default|GetHealthBar))))
  (Progress|SetPercent (Variables|/Game/Widgets/Enemies/WB_MeleeEnemy.WB_MeleeEnemy_C|GetHealthBar _aswb_melee_enemy) (/ (Variables|Default|GetEnemy_Health) 5e+01)))

(event EventAttack
  ;[1 0 0.7954] Ataque
  (Animation|Montage|PlayMontage (Variables|Character|GetMesh) "/Game/Enemies/BaseEnemy/Animations/Enemy1/Anim_BP/AM_Attack.AM_Attack"
    (:then
      (bind _asaicontroller_base_enemy (Utilities|Casting|CastToAIController_BaseEnemy (AI|GetAIController self)))
      (bind _attack_target (Variables|/Game/Enemies/BaseEnemy/AI/AIController_BaseEnemy.AIController_BaseEnemy_C|GetAttack%20Target _asaicontroller_base_enemy)
        (:then
          (Game|Damage|ApplyDamage _attack_target (Variables|Default|GetEnemy_Dmg) 0 0))
        (:else)))
    (:OnCompleted
      (Default|CallAttackEnd :!label _label))
    (:OnInterrupted
      (goto _label))))

(event Game|Damage|EventAnyDamage
  (params (Damage :type Float%20%28single-precision%29) (DamageType :type Damage%20Type%20Object%20Reference) (InstigatedBy :type Controller%20Object%20Reference) (DamageCauser :type Actor%20Object%20Reference))
  ;[1 0.01675 0] Recibir daño
  (CallFunction|MakeFloatingNumbers (Transformation|GetActorLocation) (Math|Float|Truncate Damage))
  (bind _output_get (Variables|Default|SetEnemy_Health (- (Variables|Default|GetEnemy_Health) Damage)))
  (bind _asbp_axololt (Utilities|Casting|CastToBP_Axololt (Game|GetPlayerCharacter 0)))
  (Character|LaunchCharacter (Math|Vector|MakeVector (.x (* (Math|Vector|GetForwardVector (Transformation|GetWorldRotation (Variables|/Script/Engine.Actor|GetRootComponent _asbp_axololt))) (Variables|Default|GetLaunch_Force))) (.y (* (Math|Vector|GetForwardVector (Transformation|GetWorldRotation (Variables|/Script/Engine.Actor|GetRootComponent _asbp_axololt))) (Variables|Default|GetLaunch_Force))) 0.0) false false)
  (if (<= _output_get 0.0)
    (Variables|Default|SetbUseControllerRotationYaw false)
    (Pawn|Components|CharacterMovement|DisableMovement (Variables|Character|GetCharacterMovement))
    (Animation|Montage|PlayMontage (Variables|Character|GetMesh) "/Game/Enemies/BaseEnemy/Animations/Enemy1/Anim_BP/AM_Death.AM_Death"
      (:then
        (Utilities|FlowControl|Delay 2.0)
        (Actor|DestroyActor)))))

(fn ConstructionScript
  (|CallParentFunction))

(fn GetHealth
  (return 0.0))

(fn SetMovementSpeed
  (params (Speed :type E_MovementSpeed%20Enum :default "NewEnumerator0"))
  (return 0.0))