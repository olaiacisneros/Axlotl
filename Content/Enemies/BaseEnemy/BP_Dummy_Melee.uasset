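; BP_Dummy_Melee is a melee enemy dummy that takes damage but never dies, refilling its health whenever it runs out.
; On BeginPlay it snaps the Esqueleto component to the mesh's head socket.
; Attack is empty, and the montage-driven damage and health bar update logic are left disconnected.
; The health, speed, range and patrol functions are stubs returning zero or nothing.
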(event EventBeginPlay
  ;[0.09435 1 0.07239] BeginPlay
  (Transformation|AttachComponentToComponent (Variables|Default|GetEsqueleto) (Variables|Character|GetMesh) "HeadSocket" "SnapToTarget" "SnapToTarget" "SnapToTarget" true))

(event Collision|EventActorBeginOverlap
  (params (OtherActor :type Actor%20Object%20Reference)))

(event EventTick
  (params (DeltaSeconds :type Float%20%28single-precision%29))
  ;[1 0.9142 0.2333] Event tick
)

(event EventAttack
  ;[1 0 0.8377] Ataque
)

(event Game|Damage|EventAnyDamage
  (params (Damage :type Float%20%28single-precision%29) (DamageType :type Damage%20Type%20Object%20Reference) (InstigatedBy :type Controller%20Object%20Reference) (DamageCauser :type Actor%20Object%20Reference))
  ;[1 0 0] Recibir daño
  (bind _output_get (Variables|Default|SetEnemy_Health (- (Variables|Default|GetEnemy_Health) Damage)))
  (if (<= _output_get 0.0)
    (Variables|Default|SetEnemy_Health 1e+02)))

(fn ConstructionScript
  (|CallParentFunction))

(fn GetHealth
  (return 0.0))

(fn SetMovementSpeed
  (params (Speed :type E_MovementSpeed%20Enum :default "NewEnumerator0"))
  (return 0.0))

(fn GetIdealRange
  (return 0.0 0.0))

(fn GetSplinePatrol
  (return 0))