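; BP_BaseEnemy is a base enemy character with health, combat ranges, a patrol route and selectable movement speeds.
; Any damage subtracts from its health, and at zero or below it flags itself dead and is destroyed immediately.
; Functions expose health, fixed attack and defend radii and the patrol route, and map a speed state from idle to sprint onto the CharacterMovement walk speed.
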(event EventBeginPlay)

(event Collision|EventActorBeginOverlap
  (params (OtherActor :type Actor%20Object%20Reference)))

(event EventTick
  (params (DeltaSeconds :type Float%20%28single-precision%29)))

(event Game|Damage|EventAnyDamage
  (params (Damage :type Float%20%28single-precision%29) (DamageType :type Damage%20Type%20Object%20Reference) (InstigatedBy :type Controller%20Object%20Reference) (DamageCauser :type Actor%20Object%20Reference))
  (bind _output_get (Variables|Default|SetEnemy_Health (- (Variables|Default|GetEnemy_Health) Damage)))
  (if (<= _output_get 0.0)
    (Variables|Default|SetIsDead true)
    (Actor|DestroyActor)))

(fn ConstructionScript)

(fn GetHealth
  (return (Variables|Default|GetEnemy_Health)))

(fn GetIdealRange
  (return 1.5e+02 3.5e+02))

(fn GetSplinePatrol
  (return (Variables|AI|GetPatrolRoute)))

(fn SetMovementSpeed
  (params (Speed :type E_MovementSpeed%20Enum :default "NewEnumerator0"))
  (bind _output_get (Variables|/Script/Engine.CharacterMovementComponent|SetMaxWalkSpeed (Variables|Character|GetCharacterMovement) (Utilities|Select :Index Speed :NewEnumerator0 0.0 :NewEnumerator1 1e+02 :NewEnumerator3 3e+02 :NewEnumerator2 5e+02)))
  (return _output_get))