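; Melee enemy that attacks its AI controller's target, takes damage and is destroyed when health runs out.
; Attack plays a montage and applies fixed damage to the controller's AttackTarget as soon as playback starts, then fires AttackEnd on completion or interruption.
; AnyDamage subtracts from EnemyHealth, which Tick pushes to the health bar widget every frame, assuming a maximum of 100.
; GetHealth is a stub that returns zero.
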(event EventBeginPlay)

(event Collision|EventActorBeginOverlap
  (params (OtherActor :type Actor%20Object%20Reference)))

(event EventTick
  (params (DeltaSeconds :type Float%20%28single-precision%29))
  (bind _aswb_melee_enemy (Utilities|Casting|CastToWB_MeleeEnemy (UserInterface|GetWidget (Variables|Default|GetHealthBar))))
  (Progress|SetPercent (Variables|/Game/Widgets/Enemies/WB_MeleeEnemy.WB_MeleeEnemy_C|GetHealthBar _aswb_melee_enemy) (/ (Variables|Default|GetEnemy_Health) 1e+02)))

(event EventAttack
  (Animation|Montage|PlayMontage (Variables|Character|GetMesh) "/Game/Player/Animations/AttackMontage.AttackMontage"
    (:then
      (bind _asaicontroller_base_enemy (Utilities|Casting|CastToAIController_BaseEnemy (AI|GetAIController self)))
      (bind _attack_target (Variables|/Game/Enemies/BaseEnemy/AI/AIController_BaseEnemy.AIController_BaseEnemy_C|GetAttack%20Target _asaicontroller_base_enemy)
        (:then
          (Game|Damage|ApplyDamage _attack_target 25.0 0 0))
        (:else)))
    (:OnCompleted
      (Default|CallAttackEnd :!label _label))
    (:OnInterrupted
      (goto _label))))

(event Game|Damage|EventAnyDamage
  (params (Damage :type Float%20%28single-precision%29) (DamageType :type Damage%20Type%20Object%20Reference) (InstigatedBy :type Controller%20Object%20Reference) (DamageCauser :type Actor%20Object%20Reference))
  ;[1 1 1] AnyDamage
  (bind _output_get (Variables|Default|SetEnemy_Health (- (Variables|Default|GetEnemy_Health) Damage)))
  (if (<= _output_get 0.0)
    (Actor|DestroyActor)))

(fn ConstructionScript
  (|CallParentFunction))

(fn GetHealth
  (return 0.0))