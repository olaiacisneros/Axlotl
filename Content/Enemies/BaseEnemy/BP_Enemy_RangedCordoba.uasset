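; Ranged enemy character that constantly turns to face the player and fires projectiles at its AI controller's attack target.
; Tick updates the health bar widget and player distance; Attack plays a montage, spawns the projectile from Lanzador and signals attack end.
; Damage shows floating numbers and knocks it along the player's forward vector; at zero health it plays death once, then destroys itself.
; Getter and speed functions expose ranges, distance and movement tiers.
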(event OnComponentBeginOverlap(Trigger_Deteccion)
  (params (OverlappedComponent :type Primitive%20Component%20Object%20Reference) (OtherActor :type Actor%20Object%20Reference) (OtherComp :type Primitive%20Component%20Object%20Reference) (OtherBodyIndex :type Integer) (bFromSweep :type Boolean) (SweepResult :type Hit%20Result%20Structure%20%28by%20ref%29))
  ;[1 1 1] Detecta al personaje en un radio
  (if (Actor|ActorHasTag OtherActor "Player")
    (Transformation|SetWorldRotation (Variables|Default|GetCapsuleComponent) (Math|Rotator|FindLookatRotation (Transformation|GetWorldLocation (Variables|Default|GetCapsuleComponent)) (Transformation|GetActorLocation)) false false)))

(event EventBeginPlay
  ;[0.09435 1 0.07239] BeginPlay
  (Transformation|AttachComponentToComponent (Variables|Default|GetEsqueleto) (Variables|Character|GetMesh) "HeadSocket" "SnapToTarget" "SnapToTarget" "SnapToTarget" true)
  (bind _asbp_axololt (Utilities|Casting|CastToBP_Axololt (Game|GetPlayerCharacter 0)))
  (Variables|Default|SetChar%20REF _asbp_axololt))

(event Collision|EventActorBeginOverlap
  (params (OtherActor :type Actor%20Object%20Reference)))

(event EventTick
  (params (DeltaSeconds :type Float%20%28single-precision%29))
  (bind _returnvalue (Game|GetPlayerCharacter 0))
  ;[1 0.9288 0.2916] Event tick
  (bind _aswb_ranged_enemy (Utilities|Casting|CastToWB_RangedEnemy (UserInterface|GetWidget (Variables|Default|GetHealthBar))))
  (Progress|SetPercent (Variables|/Game/Widgets/Enemies/WB_RangedEnemy.WB_RangedEnemy_C|GetHealthBar _aswb_ranged_enemy) (/ (Variables|Default|GetEnemy_Health) 1e+02))
  (Variables|Default|SetCurrent%20Distance (Math|Vector|Distance(Vector) (Transformation|GetActorLocation) (Transformation|GetActorLocation _returnvalue)))
  (Transformation|SetWorldRotation (Variables|Default|GetCapsuleComponent) (Math|Rotator|FindLookatRotation (Transformation|GetWorldLocation (Variables|Default|GetCapsuleComponent)) (Transformation|GetActorLocation _returnvalue)) false false))

(event EventAttack
  ;[1 0 0.8928] Ataque
  ;;[1 1 1] Animacion de Ataque rango
  (Animation|Montage|PlayMontage (Variables|Character|GetMesh) "/Game/Enemies/BaseEnemy/Animations/RangedEnemy/Ranged_EnemyAttack.Ranged_EnemyAttack"
    (:then
      (bind _asaicontroller_base_enemy (Utilities|Casting|CastToAIController_BaseEnemy (AI|GetAIController self)))
      (bind _attack_target (Variables|/Game/Enemies/BaseEnemy/AI/AIController_BaseEnemy.AIController_BaseEnemy_C|GetAttack%20Target _asaicontroller_base_enemy)
        (:then
          (Game|SpawnActorfromClass "/Game/Actors/BP_ProjectileEnemy3.BP_ProjectileEnemy3_C" (Transformation|GetWorldTransform (Variables|Default|GetLanzador)) "Undefined" "MultiplyWithRoot" 0 0))
        (:else)))
    (:OnCompleted
      (Default|CallAttackEnd :!label _label))
    (:OnInterrupted
      (goto _label))))

(event Game|Damage|EventAnyDamage
  (params (Damage :type Float%20%28single-precision%29) (DamageType :type Damage%20Type%20Object%20Reference) (InstigatedBy :type Controller%20Object%20Reference) (DamageCauser :type Actor%20Object%20Reference))
  ;[1 0.01553 0] Recibir daño
  (CallFunction|MakeFloatingNumbers (Transformation|GetActorLocation) (Math|Float|Truncate Damage))
  (Variables|Default|SetCanBeHit false)
  (bind _output_get (Variables|Default|SetEnemy_Health (- (Variables|Default|GetEnemy_Health) Damage)))
  (Transformation|SetWorldRotation (Variables|Default|GetCapsuleComponent) (Math|Rotator|FindLookatRotation (Transformation|GetWorldLocation (Variables|Default|GetCapsuleComponent)) (Transformation|GetActorLocation (Game|GetPlayerCharacter 0))) false false)
  (bind _asbp_axololt (Utilities|Casting|CastToBP_Axololt (Game|GetPlayerCharacter 0)))
  (Character|LaunchCharacter (Math|Vector|MakeVector (.x (* (Math|Vector|GetForwardVector (Transformation|GetWorldRotation (Variables|/Script/Engine.Actor|GetRootComponent _asbp_axololt))) (Variables|Default|GetLaunchForce))) (.y (* (Math|Vector|GetForwardVector (Transformation|GetWorldRotation (Variables|/Script/Engine.Actor|GetRootComponent _asbp_axololt))) (Variables|Default|GetLaunchForce))) 0.0) false false)
  (if (<= _output_get 0.0)
    (Utilities|FlowControl|DoOnce false
      (:Completed
        (Variables|Default|SetbUseControllerRotationYaw false)
        (Pawn|Components|CharacterMovement|DisableMovement (Variables|Character|GetCharacterMovement))
        (Audio|SpawnSoundAttached "/Game/Audio/SFX/Player/Weapon1/Collision/Blueprint/MS_ImpactSlime.MS_ImpactSlime" (Variables|Character|GetMesh) "None" "0, 0, 0" "0, 0, 0" "KeepRelativeOffset" false 1.0 1.0 0.0 0 0)
        (Animation|Montage|PlayMontage (Variables|Character|GetMesh) "/Game/Enemies/BaseEnemy/Animations/Enemy1/Anim_BP/AM_Death.AM_Death"
          (:then
            (Utilities|FlowControl|Delay 3.0)
            (Actor|DestroyActor)))))))

(fn ConstructionScript
  (|CallParentFunction))

(fn SetMovementSpeed
  (params (Speed :type E_MovementSpeed%20Enum :default "NewEnumerator0"))
  (bind _output_get (Variables|/Script/Engine.CharacterMovementComponent|SetMaxWalkSpeed (Variables|Character|GetCharacterMovement) (Utilities|Select :Index Speed :NewEnumerator0 0.0 :NewEnumerator1 2e+02 :NewEnumerator3 3e+02 :NewEnumerator2 5e+02)))
  (return _output_get))

(fn GetIdealRange
  (return (Variables|Default|GetEnemy_Attack_Range) 6e+02))

(fn GetMaxDistance
  (return (Variables|Default|GetMaxEscapeDistance)))

(fn GetCurrentPosition
  (return (Variables|Default|GetCurrent%20Distance)))