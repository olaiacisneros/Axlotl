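; Player axolotl Blueprint with dash, ranged or melee attacks, interface-based interaction with overlapping actors, and a pause menu.
; BeginPlay creates the health HUD, restores health, room count and weapon from GI_Variables, and binds events that write changes back.
; Dashing while moving briefly hides the mesh behind a Niagara effect; light attack fires a projectile or plays melee animation by weapon enum.
; Damage, weapon-toggle and run/idle animation logic is disconnected.
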(event Custom|UpdateRooms_Event
  (params (Rooms :type Float%20%28double-precision%29))
  (bind _output_get (Variables|/Game/Instances/GI_Variables.GI_Variables_C|SetRoom_Counter (Variables|Default|GetAs%20GI%20Variables) Rooms)))

(event Custom|UpdateHealth_Event
  (params (Health :type Float%20%28double-precision%29))
  (bind _output_get (Variables|/Game/Instances/GI_Variables.GI_Variables_C|SetHealth (Variables|Default|GetAs%20GI%20Variables) Health)))

(event Custom|UpdateWeaponChoice_Event
  (params (Weapon :type Float%20%28double-precision%29))
  (bind _output_get (Variables|/Game/Instances/GI_Variables.GI_Variables_C|SetWeaponSelected (Variables|Default|GetAs%20GI%20Variables) Weapon)))

(event Input|EnhancedActionEvents|EnhancedInputActionLAttackAction
  (params (ActionValue :type Boolean) (ElapsedSeconds :type Float%20%28double-precision%29) (TriggeredSeconds :type Float%20%28double-precision%29) (InputAction :type Input%20Action%20Object%20Reference :default "/Game/Player/Input/Actions/LAttackAction.LAttackAction"))
  ;[1 1 1] Light Attack
  (switch Utilities|FlowControl|Switch|SwitchonEnum_Weapons (Variables|Default|GetEnum_weapons)
    (:NewEnumerator0
      (Class|Axololt|RangedAttack)
      (Transformation|SetRelativeRotation (Variables|Default|GetSpawn%20Transform) (Variables|Default|GetRotatorProjectile) false false)
      (Game|SpawnActorfromClass "/Game/Player/Actors/BP_Axolotl_Projectile.BP_Axolotl_Projectile_C" (Transformation|GetWorldTransform (Variables|Default|GetSpawn%20Transform)) "Undefined" "MultiplyWithRoot" 0 self))
    (:NewEnumerator1
      (Components|Animation|PlayAnimation (Variables|Character|GetMesh) "/Game/Animations_Axolot/Animaciones/Ataque_basico_melee.Ataque_basico_melee" false))))

(event Input|EnhancedActionEvents|EnhancedInputActionMoveAction
  (params (ActionValue :type Vector%202D%20Structure) (ElapsedSeconds :type Float%20%28double-precision%29) (TriggeredSeconds :type Float%20%28double-precision%29) (InputAction :type Input%20Action%20Object%20Reference :default "/Game/Player/Input/Actions/MoveAction.MoveAction"))
  (:Triggered
    (Variables|Default|SetMoving true))
  (:Ongoing
    (Variables|Default|SetMoving true))
  (:Canceled
    (Variables|Default|SetMoving false :!label _label)
    (Audio|Components|Audio|Stop (Variables|Character|GetMesh)))
  (:Completed
    (goto _label)))

(event Input|EnhancedActionEvents|EnhancedInputActionHAttackAction
  (params (ActionValue :type Boolean) (ElapsedSeconds :type Float%20%28double-precision%29) (TriggeredSeconds :type Float%20%28double-precision%29) (InputAction :type Input%20Action%20Object%20Reference :default "/Game/Player/Input/Actions/HAttackAction.HAttackAction"))
  ;[1 1 1] Hard Attack
  (if (not (Variables|Default|GetRanged))
    (Components|Animation|PlayAnimation (Variables|Character|GetMesh) "/Game/Animations_Axolot/Animaciones/Ataque_fuerte_melee.Ataque_fuerte_melee" false)))

(event Input|EnhancedActionEvents|EnhancedInputActionChangeRanged
  (params (ActionValue :type Boolean) (ElapsedSeconds :type Float%20%28double-precision%29) (TriggeredSeconds :type Float%20%28double-precision%29) (InputAction :type Input%20Action%20Object%20Reference :default "/Game/Player/Input/Actions/ChangeRanged.ChangeRanged"))
  ;[1 1 1] ChangeRanged
)

(event Input|EnhancedActionEvents|EnhancedInputActionDashAction
  (params (ActionValue :type Boolean) (ElapsedSeconds :type Float%20%28double-precision%29) (TriggeredSeconds :type Float%20%28double-precision%29) (InputAction :type Input%20Action%20Object%20Reference :default "/Game/Player/Input/Actions/DashAction.DashAction"))
  (bind _sp_dash_vfx (Variables|Default|GetSP_Dash_VFX))
  (Variables|Default|SetDash ActionValue)
  (if (Variables|Default|GetMoving)
    (Rendering|SetVisibility (Variables|Character|GetMesh) false false)
    (Niagara|SpawnSystemAttached "/Game/VFX/NS_Dash.NS_Dash" _sp_dash_vfx "None" (Transformation|GetWorldLocation _sp_dash_vfx) (Math|Rotator|MakeRotator 0.0 0.0 (.yaw (Math|Conversions|RotationFromXVector (Transformation|GetActorForwardVector)))) "KeepWorldPosition" true)
    (Utilities|FlowControl|Delay 0.4)
    (Rendering|SetVisibility (Variables|Character|GetMesh) true false)
    (Variables|Default|SetDash false)))

(event Input|EnhancedActionEvents|EnhancedInputActionPauseGame
  (params (ActionValue :type Boolean) (ElapsedSeconds :type Float%20%28double-precision%29) (TriggeredSeconds :type Float%20%28double-precision%29) (InputAction :type Input%20Action%20Object%20Reference :default "/Game/Player/Input/Actions/PauseGame.PauseGame"))
  (bind _returnvalue (Game|GetPlayerController 0))
  ;[1 1 1] Pausar juego
  (:Started
    (if (not (Variables|Default|GetPauseMenu))
      (Variables|Default|SetPauseMenu true)
      (bind _returnvalue_2 (UserInterface|CreateWidget "/Game/Widgets/WB_PauseMenu.WB_PauseMenu_C" _returnvalue))
      (bind _output_get (Variables|Default|SetPauseMenuWidget _returnvalue_2))
      (UserInterface|Viewport|AddtoViewport _output_get 0)
      (Input|SetInputModeGameandUI _returnvalue (Variables|Default|GetPauseMenuWidget) "DoNotLock" true false)
      (Variables|/Script/Engine.PlayerController|SetbShowMouseCursor (Game|GetPlayerController 0) true)
      (Game|SetGamePaused true)
      (else
        (Variables|Default|SetPauseMenu false)
        (Widget|RemovefromParent (Variables|Default|GetPauseMenuWidget))
        (Game|SetGamePaused false)
        (Input|SetInputModeGameOnly _returnvalue false)
        (Variables|/Script/Engine.PlayerController|SetbShowMouseCursor (Game|GetPlayerController 0) false)))))

(event Input|EnhancedActionEvents|EnhancedInputActionInteractuar
  (params (ActionValue :type Boolean) (ElapsedSeconds :type Float%20%28double-precision%29) (TriggeredSeconds :type Float%20%28double-precision%29) (InputAction :type Input%20Action%20Object%20Reference :default "/Game/Player/Input/Actions/Interactuar.Interactuar"))
  ;[1 1 1] Cambio de arma
  (bind _array_element (Utilities|Array|ForEachLoopwithBreak (Collision|GetOverlappingActors "/Script/Engine.Actor" :!class /Script/Engine.Actor))
    (:LoopBody
      (if (Utilities|DoesObjectImplementInterface _array_element "/Game/Interface/Interactable.Interactable_C")
        (Class|Interactable|Interactable(Message) _array_element)))))

(event Input|EnhancedActionEvents|EnhancedInputActionInteractuar
  (params (ActionValue :type Boolean) (ElapsedSeconds :type Float%20%28double-precision%29) (TriggeredSeconds :type Float%20%28double-precision%29) (InputAction :type Input%20Action%20Object%20Reference :default "/Game/Player/Input/Actions/Interactuar.Interactuar")))

(event EventBeginPlay
  (bind _returnvalue (UserInterface|CreateWidget "/Game/Widgets/WB_Player.WB_Player_C"))
  (bind _output_get (Variables|Default|SetUI_HealthBar _returnvalue))
  (UserInterface|Viewport|AddtoViewport _output_get 0)
  (bind _asgi_variables (Utilities|Casting|CastToGI_Variables (Game|GetGameInstance)))
  (bind _output_get_2 (Variables|Default|SetAs%20GI%20Variables _asgi_variables))
  (Default|SaveVariables _output_get_2)
  (Input|EnableInput (Game|GetPlayerController 0))
  (EventDispatchers|BindEventtoUpdateRooms (delegate Custom|UpdateRooms_Event))
  (Variables|Default|SetRoom%20Counter (stale Custom|UpdateRooms_Event _output_get))
  (EventDispatchers|BindEventtoUpdateHealth (delegate Custom|UpdateHealth_Event))
  (Variables|Default|SetHealth (stale Custom|UpdateHealth_Event _output_get))
  (EventDispatchers|BindEventtoUpdateWeaponChoice (delegate Custom|UpdateWeaponChoice_Event))
  (bind _output_get_3 (Variables|Default|SetWeaponSelected (stale Custom|UpdateWeaponChoice_Event _output_get)))
  (if (== _output_get_3 0.0)
    (Variables|Default|SetEnum_weapons "NewEnumerator0")
    (else
      (Variables|Default|SetEnum_weapons "NewEnumerator1"))))

(event EventTick
  (params (DeltaSeconds :type Float%20%28single-precision%29))
  (Default|UpdateHealth (Variables|Default|GetUI_HealthBar) (Variables|Default|GetHealth)))

(event Game|Damage|EventAnyDamage
  (params (Damage :type Float%20%28single-precision%29) (DamageType :type Damage%20Type%20Object%20Reference) (InstigatedBy :type Controller%20Object%20Reference) (DamageCauser :type Actor%20Object%20Reference))
  ;[1 1 1] Apply damage
)

(fn ConstructionScript)