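; BP_Enemy1 is an AI enemy character that spots the Axololt pawn and attacks it in melee.
; Pawn sensing sets the HasSeenPlayer blackboard key on sight, and nothing here clears it.
; MeleeAttack sphere-traces forward, and only on an Axololt hit plays a montage, applies damage and halts walking for a second.
; The attack still draws its debug trace and prints a message on hit.
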(event OnSeePawn(PawnSensing)
  (params (Pawn :type Pawn%20Object%20Reference))
  (Utilities|Casting|CastToAxololt Pawn)
  (AI|Components|Blackboard|SetValueasBool (AI|GetBlackboard (AI|GetAIController self)) (Utilities|Name|MakeLiteralName "HasSeenPlayer") true))

(event Custom|MeleeAttack
  (bind _returnvalue (Transformation|GetActorLocation))
  (bind _charactermovement (Variables|Character|GetCharacterMovement))
  (bind (_outhit _returnvalue_2) (Collision|SphereTraceForObjects _returnvalue (+ _returnvalue (* (Math|Vector|GetForwardVector (Transformation|GetActorRotation)) 2.5e+02)) 1.2e+02 (Utilities|Array|MakeArray "ObjectTypeQuery3") false 0 "ForDuration"))
  (if _returnvalue_2
    (bind _asaxololt (Utilities|Casting|CastToAxololt (.HitActor (Collision|BreakHitResult _outhit))))
    (Development|PrintString "Attack")
    (Animation|PlayAnimMontage "/Game/AI/Enemy1/Animations/Anim_Enemy1.Anim_Enemy1" 1.0 "None")
    (Game|Damage|ApplyDamage _asaxololt (Variables|Default|GetAttack_Dmg) 0 0)
    (Variables|/Script/Engine.CharacterMovementComponent|SetMaxWalkSpeed _charactermovement 0.0)
    (Utilities|FlowControl|Delay 1.0)
    (Variables|/Script/Engine.CharacterMovementComponent|SetMaxWalkSpeed _charactermovement (Variables|Default|GetEnemy_Speed))))

(event EventBeginPlay)

(event Collision|EventActorBeginOverlap
  (params (OtherActor :type Actor%20Object%20Reference)))

(event EventTick
  (params (DeltaSeconds :type Float%20%28single-precision%29)))

(fn ConstructionScript)