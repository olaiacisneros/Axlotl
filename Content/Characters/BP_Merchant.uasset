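; BP_Merchant is a merchant character whose Interactable event toggles the WB_Merchant widget using an Open flag.
; Opening constructs a new widget, adds it to the viewport, shows the mouse cursor and sets UI-only input focused on it.
; Closing restores game-only input, removes the widget and forces garbage collection, but leaves the cursor flag enabled.
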(event Custom|Open%20Widget
  (bind _returnvalue (Game|GetPlayerController 0))
  (bind _returnvalue_2 (Game|ConstructObjectfromClass "/Game/Widgets/Merchant/WB_Merchant.WB_Merchant_C"))
  (bind _output_get (Variables|Default|SetWB%20Merchant _returnvalue_2))
  (UserInterface|Viewport|AddtoViewport _output_get 0)
  (Variables|/Script/Engine.PlayerController|SetbShowMouseCursor _returnvalue true)
  (Input|SetInputModeUIOnly _returnvalue (Variables|Default|GetWB%20Merchant) "DoNotLock" true)
  (Variables|Default|SetOpen true))

(event Custom|Close%20Widget
  (Input|SetInputModeGameOnly 0 true)
  (Widget|RemovefromParent (Variables|Default|GetWB%20Merchant))
  (Utilities|Platform|CollectGarbage)
  (Variables|Default|SetOpen false))

(event EventInteractable
  (if (Variables|Default|GetOpen)
    (CallFunction|CloseWidget)
    (else
      (CallFunction|OpenWidget))))

(fn ConstructionScript)