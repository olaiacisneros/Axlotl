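; GI_Music is a music manager, named as a Game Instance, that switches between menu, battle, merchant and boss tracks.
; Each event spawns a 2D sound, tracking it with a component reference and playing flag, after fading or stopping another track through nested validity checks.
; No event stops merchant music, and the menu event leaves battle and boss flags set.
; Separately, BeginTime stores a start timestamp and TimePassed prints and returns elapsed minutes.
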(event Custom|Spawn_battleMusic
  ;[1 0 0.6145] Change of Songs
  (Utilities|IsValid (Variables|Default|GetBattle_Music)
    (:Is%20Valid
      (if (not (Variables|Default|GetisPlayingBattle))
        (bind _returnvalue (Audio|SpawnSound2D "/Game/Audio/Music/Blueprints/Battle_Level/MS_Battle.MS_Battle" 1.0 1.0 0.0 0 true))
        (Variables|Default|SetBattle_Music _returnvalue)
        (Variables|Default|SetisPlayingBattle true)))
    (:Is%20Not%20Valid
      (Utilities|IsValid (Variables|Default|GetMenuMusic)
        (:Is%20Valid
          (if (Variables|Default|GetisPlayingMenu)
            (Audio|Components|Audio|FadeOut (Variables|Default|GetMenuMusic) 0.5 0.0 "Linear" :!class /Script/Engine.AudioComponent)
            (Variables|Default|SetisPlayingMenu false)
            (bind _returnvalue_2 (Audio|SpawnSound2D "/Game/Audio/Music/Blueprints/Battle_Level/MS_Battle.MS_Battle" 1.0 1.0 0.0 0 true))
            (Variables|Default|SetBattle_Music _returnvalue_2)
            (Variables|Default|SetisPlayingBattle true)
            (else
              (bind _returnvalue_3 (Audio|SpawnSound2D "/Game/Audio/Music/Blueprints/Battle_Level/MS_Battle.MS_Battle" 1.0 1.0 0.0 0 true))
              (Variables|Default|SetBattle_Music _returnvalue_3)
              (Variables|Default|SetisPlayingBattle true))))
        (:Is%20Not%20Valid
          (Utilities|IsValid (Variables|Default|GetBossMusic)
            (:Is%20Valid
              (if (Variables|Default|GetisPlayingBoss)
                (Audio|Components|Audio|Stop (Variables|Default|GetBossMusic))
                (Variables|Default|SetisPlayingBoss false)
                (bind _returnvalue_4 (Audio|SpawnSound2D "/Game/Audio/Music/Blueprints/Battle_Level/MS_Battle.MS_Battle" 1.0 1.0 0.0 0 true))
                (Variables|Default|SetBattle_Music _returnvalue_4)
                (Variables|Default|SetisPlayingBattle true)
                (else
                  (bind _returnvalue_5 (Audio|SpawnSound2D "/Game/Audio/Music/Blueprints/Battle_Level/MS_Battle.MS_Battle" 1.0 1.0 0.0 0 true))
                  (Variables|Default|SetBattle_Music _returnvalue_5)
                  (Variables|Default|SetisPlayingBattle true))))
            (:Is%20Not%20Valid
              (bind _returnvalue_6 (Audio|SpawnSound2D "/Game/Audio/Music/Blueprints/Battle_Level/MS_Battle.MS_Battle" 1.0 1.0 0.0 0 true))
              (Variables|Default|SetBattle_Music _returnvalue_6)
              (Variables|Default|SetisPlayingBattle true))))))))

(event Custom|SetNewMusicMerchant
  ;[1 0 0.6145] Change of Songs
  (Utilities|IsValid (Variables|Default|GetMerchant_Music)
    (:Is%20Valid
      (if (not (Variables|Default|GetisPlayingMerchant))
        (bind _returnvalue (Audio|SpawnSound2D "/Game/Audio/Music/Blueprints/Merchant_level/MS_Merchant.MS_Merchant" 1.0 1.0 0.0 0))
        (bind _output_get (Variables|Default|SetMerchant_Music _returnvalue))
        (Audio|Components|Audio|FadeIn _output_get 0.5 1.0 0.0 "Linear" :!class /Script/Engine.AudioComponent)
        (Variables|Default|SetisPlayingMerchant true)))
    (:Is%20Not%20Valid
      (Utilities|IsValid (Variables|Default|GetBattle_Music)
        (:Is%20Valid
          (if (Variables|Default|GetisPlayingBattle)
            (Audio|Components|Audio|FadeOut (Variables|Default|GetBattle_Music) 0.5 0.0 "Linear" :!class /Script/Engine.AudioComponent)
            (Variables|Default|SetisPlayingBattle false)
            (bind _returnvalue_2 (Audio|SpawnSound2D "/Game/Audio/Music/Blueprints/Merchant_level/MS_Merchant.MS_Merchant" 1.0 1.0 0.0 0))
            (bind _output_get_2 (Variables|Default|SetMerchant_Music _returnvalue_2))
            (Audio|Components|Audio|FadeIn _output_get_2 0.5 1.0 0.0 "Linear" :!class /Script/Engine.AudioComponent)
            (Variables|Default|SetisPlayingMerchant true)
            (else
              (bind _returnvalue_3 (Audio|SpawnSound2D "/Game/Audio/Music/Blueprints/Merchant_level/MS_Merchant.MS_Merchant" 1.0 1.0 0.0 0))
              (Variables|Default|SetMerchant_Music _returnvalue_3)
              (Variables|Default|SetisPlayingMerchant true))))
        (:Is%20Not%20Valid
          (Utilities|IsValid (Variables|Default|GetMenuMusic)
            (:Is%20Valid
              (if (Variables|Default|GetisPlayingMenu)
                (Audio|Components|Audio|FadeOut (Variables|Default|GetMenuMusic) 0.5 0.0 "Linear" :!class /Script/Engine.AudioComponent)
                (Variables|Default|SetisPlayingMenu false)
                (bind _returnvalue_4 (Audio|SpawnSound2D "/Game/Audio/Music/Blueprints/Merchant_level/MS_Merchant.MS_Merchant" 1.0 1.0 0.0 0))
                (Variables|Default|SetMerchant_Music _returnvalue_4)
                (Variables|Default|SetisPlayingMerchant true)
                (else
                  (bind _returnvalue_5 (Audio|SpawnSound2D "/Game/Audio/Music/Blueprints/Merchant_level/MS_Merchant.MS_Merchant" 1.0 1.0 0.0 0))
                  (Variables|Default|SetMerchant_Music _returnvalue_5)
                  (Variables|Default|SetisPlayingMerchant true))))
            (:Is%20Not%20Valid
              (Utilities|IsValid (Variables|Default|GetBossMusic)
                (:Is%20Valid
                  (if (Variables|Default|GetisPlayingBoss)
                    (Audio|Components|Audio|FadeOut (Variables|Default|GetBossMusic) 0.5 0.0 "Linear" :!class /Script/Engine.AudioComponent)
                    (Variables|Default|SetisPlayingBoss false)
                    (bind _returnvalue_6 (Audio|SpawnSound2D "/Game/Audio/Music/Blueprints/Merchant_level/MS_Merchant.MS_Merchant" 1.0 1.0 0.0 0))
                    (Variables|Default|SetMerchant_Music _returnvalue_6)
                    (Variables|Default|SetisPlayingMerchant true)
                    (else
                      (bind _returnvalue_7 (Audio|SpawnSound2D "/Game/Audio/Music/Blueprints/Merchant_level/MS_Merchant.MS_Merchant" 1.0 1.0 0.0 0))
                      (Variables|Default|SetMerchant_Music _returnvalue_7)
                      (Variables|Default|SetisPlayingMerchant true))))
                (:Is%20Not%20Valid
                  (bind _returnvalue_8 (Audio|SpawnSound2D "/Game/Audio/Music/Blueprints/Merchant_level/MS_Merchant.MS_Merchant" 1.0 1.0 0.0 0))
                  (Variables|Default|SetMerchant_Music _returnvalue_8)
                  (Variables|Default|SetisPlayingMerchant true))))))))))

(event Custom|SetNewMusicBoss
  ;[1 0 0.6145] Change of Songs
  (Utilities|IsValid (Variables|Default|GetBossMusic)
    (:Is%20Valid
      (if (not (Variables|Default|GetisPlayingBoss))
        (bind _returnvalue (Audio|SpawnSound2D "/Game/Audio/Music/Blueprints/Boss_Level/MS_Boss.MS_Boss" 1.0 1.0 0.0 0))
        (Variables|Default|SetBossMusic _returnvalue)
        (Variables|Default|SetisPlayingBoss true)))
    (:Is%20Not%20Valid
      (Utilities|IsValid (Variables|Default|GetBattle_Music)
        (:Is%20Valid
          (if (Variables|Default|GetisPlayingBattle)
            (Audio|Components|Audio|FadeOut (Variables|Default|GetBattle_Music) 0.5 0.0 "Linear" :!class /Script/Engine.AudioComponent)
            (Variables|Default|SetisPlayingBattle false)
            (bind _returnvalue_2 (Audio|SpawnSound2D "/Game/Audio/Music/Blueprints/Boss_Level/MS_Boss.MS_Boss" 1.0 1.0 0.0 0))
            (Variables|Default|SetBossMusic _returnvalue_2)
            (Variables|Default|SetisPlayingBoss true)
            (else
              (bind _returnvalue_3 (Audio|SpawnSound2D "/Game/Audio/Music/Blueprints/Boss_Level/MS_Boss.MS_Boss" 1.0 1.0 0.0 0))
              (Variables|Default|SetBossMusic _returnvalue_3)
              (Variables|Default|SetisPlayingBoss true))))
        (:Is%20Not%20Valid
          (Utilities|IsValid (Variables|Default|GetMenuMusic)
            (:Is%20Valid
              (if (Variables|Default|GetisPlayingMenu)
                (Audio|Components|Audio|FadeOut (Variables|Default|GetMenuMusic) 0.5 0.0 "Linear" :!class /Script/Engine.AudioComponent)
                (Variables|Default|SetisPlayingMenu false)
                (bind _returnvalue_4 (Audio|SpawnSound2D "/Game/Audio/Music/Blueprints/Boss_Level/MS_Boss.MS_Boss" 1.0 1.0 0.0 0))
                (Variables|Default|SetBossMusic _returnvalue_4)
                (Variables|Default|SetisPlayingBoss true)
                (else
                  (bind _returnvalue_5 (Audio|SpawnSound2D "/Game/Audio/Music/Blueprints/Boss_Level/MS_Boss.MS_Boss" 1.0 1.0 0.0 0))
                  (Variables|Default|SetBossMusic _returnvalue_5)
                  (Variables|Default|SetisPlayingBoss true))))
            (:Is%20Not%20Valid
              (bind _returnvalue_6 (Audio|SpawnSound2D "/Game/Audio/Music/Blueprints/Boss_Level/MS_Boss.MS_Boss" 1.0 1.0 0.0 0))
              (Variables|Default|SetBossMusic _returnvalue_6)
              (Variables|Default|SetisPlayingBoss true))))))))

(event Custom|SpawnMenuMusic
  ;[1 0 0.6145] Change of Songs
  (Utilities|IsValid (Variables|Default|GetMenuMusic)
    (:Is%20Valid
      (if (not (Variables|Default|GetisPlayingMenu))
        (bind _returnvalue (Audio|SpawnSound2D "/Game/Audio/Music/Blueprints/Main_Menu/MS_Menu.MS_Menu" 1.0 1.0 0.0 0 true))
        (Variables|Default|SetMenuMusic _returnvalue)
        (Variables|Default|SetisPlayingMenu true)))
    (:Is%20Not%20Valid
      (Utilities|IsValid (Variables|Default|GetBattle_Music)
        (:Is%20Valid
          (if (Variables|Default|GetisPlayingBattle)
            (Audio|Components|Audio|Stop (Variables|Default|GetBattle_Music))
            (bind _returnvalue_2 (Audio|SpawnSound2D "/Game/Audio/Music/Blueprints/Main_Menu/MS_Menu.MS_Menu" 1.0 1.0 0.0 0 true))
            (Variables|Default|SetMenuMusic _returnvalue_2)
            (Variables|Default|SetisPlayingMenu true)
            (else
              (bind _returnvalue_3 (Audio|SpawnSound2D "/Game/Audio/Music/Blueprints/Main_Menu/MS_Menu.MS_Menu" 1.0 1.0 0.0 0 true))
              (Variables|Default|SetMenuMusic _returnvalue_3)
              (Variables|Default|SetisPlayingMenu true))))
        (:Is%20Not%20Valid
          (Utilities|IsValid (Variables|Default|GetBossMusic)
            (:Is%20Valid
              (if (Variables|Default|GetisPlayingBoss)
                (Audio|Components|Audio|FadeOut (Variables|Default|GetBossMusic) 0.5 0.0 "Linear" :!class /Script/Engine.AudioComponent)
                (bind _returnvalue_4 (Audio|SpawnSound2D "/Game/Audio/Music/Blueprints/Main_Menu/MS_Menu.MS_Menu" 1.0 1.0 0.0 0 true))
                (Variables|Default|SetMenuMusic _returnvalue_4)
                (Variables|Default|SetisPlayingMenu true)
                (else
                  (bind _returnvalue_5 (Audio|SpawnSound2D "/Game/Audio/Music/Blueprints/Main_Menu/MS_Menu.MS_Menu" 1.0 1.0 0.0 0 true))
                  (Variables|Default|SetMenuMusic _returnvalue_5)
                  (Variables|Default|SetisPlayingMenu true))))
            (:Is%20Not%20Valid
              (bind _returnvalue_6 (Audio|SpawnSound2D "/Game/Audio/Music/Blueprints/Main_Menu/MS_Menu.MS_Menu" 1.0 1.0 0.0 0 true))
              (Variables|Default|SetMenuMusic _returnvalue_6)
              (Variables|Default|SetisPlayingMenu true))))))))

(event Custom|BeginTime
  (Variables|Default|SetDateTimeStart (Math|DateTime|Now))
  (Variables|Default|SetisTimeStarted true))

(fn TimePassed
  (bind _returnvalue (Math|DateTime|Now))
  (bind _datetimestart (Variables|Default|GetDateTimeStart))
  (bind _returnvalue_2 (- _returnvalue _datetimestart))
  (bind _returnvalue_3 (Math|Timespan|GetTotalMinutes _returnvalue_2))
  (Development|PrintText (Utilities|Text|FormatText "TimePassed: {0}" _returnvalue_3))
  (return _returnvalue_3))